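; BP_End is an end-of-game trigger that shows a game-over message and then loads the Assignment4 level.
; Any overlap with its Sphere spawns a BP_GameOverMsg in front of the player pawn, yawed 180 degrees from the pawn to face it.
; A timeline drives the message's opacity, then destroys the message and opens the level when finished.
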(event `self.ReceiveBeginPlay`)

(event `self.ReceiveActorBeginOverlap`
  (params (OtherActor :type "Actor Object Reference")))

(event `self.ReceiveTick`
  (params (DeltaSeconds :type "Float (single-precision)")))

(event `self.Sphere.OnComponentBeginOverlap`
  (params (OtherActor :type "Actor Object Reference") (OtherComp :type "PrimitiveComponent Object Reference") (OtherBodyIndex :type Integer) (bFromSweep :type Boolean) (SweepResult :type "EngineTypes.HitResult Structure (by ref)"))
  (bind _returnvalue (`GameplayStatics.GetPlayerPawn` 0))
  (bind _returnvalue_2 (`|SpawnActorFromClass` "/Game/Blueprints/BP_GameOverMsg.BP_GameOverMsg_C" (`KismetMathLibrary.MakeTransform` (+ (* (`self.GetActorForwardVector` _returnvalue) 400.0) (.location (`self.GetTransform` _returnvalue))) (`KismetMathLibrary.MakeRotator` (.pitch (.rotation (`self.GetTransform` _returnvalue))) (+ (.yaw (.rotation (`self.GetTransform` _returnvalue))) 180.0) (.roll (.rotation (`self.GetTransform` _returnvalue)))) (.scale (`self.GetTransform` _returnvalue)))))
  (bind (_direction _opacity) (`Timeline|Timeline_0`)
    (:`Update`
      (`/Game/Blueprints/BP_GameOverMsg.OpacityWithValue` _returnvalue_2 _opacity))
    (:`Finished`
      (`|ExecutionSequence`
        (:`then_0`
          (`self.K2_DestroyActor` _returnvalue_2))
        (:`then_1`
          (`GameplayStatics.OpenLevel` "Assignment4"))))))

(fn `UserConstructionScript`)