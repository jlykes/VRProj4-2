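; A 2.5D player character with jumping, movement along world axes and a side-on style follow camera.
; MoveRight and MoveForward inputs move the character along world X (inverted) and Y, independent of camera rotation.
; On BeginPlay the spring arm detaches, stores its world Y and enables HMD orientation following on the camera manager.
; Each Tick moves the arm to the player pawn's X and Z, keeping that initial Y depth fixed.
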(event `InputAxis|MoveRight`
  (params (AxisValue :type "Float (single-precision)"))
  ;[1 1 1] Player movement
  (`self.AddMovementInput` (-1.0 0.0 0.0) AxisValue))

(event `InputAxis|MoveForward`
  (params (AxisValue :type "Float (single-precision)"))
  ;[1 1 1] Player movement
  (`self.AddMovementInput` (0.0 1.0 0.0) AxisValue))

(event `InputAction|Jump`
  ;[1 1 1] Player movement
  (:`Pressed`
    (`self.Jump`))
  (:`Released`
    (`self.StopJumping`)))

(event `self.ReceiveBeginPlay`
  (bind (_returnvalue_x _returnvalue_y) (`KismetMathLibrary.BreakVector` (`SceneComponent.K2_GetComponentLocation` (`self.SpringArm`))))
  (`SceneComponent.DetachFromParent` (`self.SpringArm`) true)
  (set `PlayerCameraManager.bFollowHmdOrientation` true (`GameplayStatics.GetPlayerCameraManager` 0))
  (set `self.InitialWorldY` _returnvalue_y))

(event `self.ReceiveActorBeginOverlap`
  (params (OtherActor :type "Actor Object Reference")))

(event `self.ReceiveTick`
  (params (DeltaSeconds :type "Float (single-precision)"))
  (bind (_returnvalue_x _returnvalue_y _returnvalue_z) (`KismetMathLibrary.BreakVector` (`self.K2_GetActorLocation` (`GameplayStatics.GetPlayerPawn` 0))))
  (`SceneComponent.K2_SetWorldLocation` (`self.SpringArm`) (`KismetMathLibrary.MakeVector` _returnvalue_x (`self.InitialWorldY`) _returnvalue_z) false))

(fn `UserConstructionScript`)